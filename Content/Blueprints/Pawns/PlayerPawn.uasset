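; Player character with a double jump, a ground dash and a thrown knife, which also creates the cooldown HUD on BeginPlay.
; A DoN gate makes the second jump an upward launch and resets on landing.
; E launches along the stored movement axes through a DoOnce that resets after a delay begun on key release, while Tick counts Cooldown down using Delay.
; Q spawns a Knife at Arrow1 and impulses it forward.
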(event EventOnLanded
  (params (Hit :type Hit%20Result%20Structure%20%28by%20ref%29))
  (Utilities|FlowControl|DoN 2) ; enters at Reset
)

(event EventBeginPlay
  (Variables|Default|SetCooldown 0.0)
  (bind _returnvalue (UserInterface|CreateWidget "/Game/UI/CooldownHUD.CooldownHUD_C" (Game|GetPlayerController 0)))
  (UserInterface|Viewport|AddtoViewport _returnvalue 0))

(event EventTick
  (params (DeltaSeconds :type Float%20%28single-precision%29))
  (if (not (== (Variables|Default|GetCooldown) 0.0))
    (Utilities|FlowControl|Delay 1.0)
    (Variables|Default|SetCooldown (- (Variables|Default|GetCooldown) 1.0))))

(event Input|ActionEvents|InputActionJump
  (params (Key :type Key%20Structure))
  (:Pressed
    (bind _counter (Utilities|FlowControl|DoN 2)
      (:Exit
        (switch int _counter
          (:1
            (Character|Jump))
          (:2
            (Character|LaunchCharacter "0, 0,1000.000000" false true)))))))

(event Input|AxisEvents|InputAxisMoveRight
  (params (AxisValue :type Float%20%28single-precision%29))
  (Variables|Default|SetRight/LeftMovement AxisValue))

(event Input|AxisEvents|InputAxisMoveForward
  (params (AxisValue :type Float%20%28single-precision%29))
  (Variables|Default|SetForward/BackwardMovement AxisValue))

(event Input|KeyboardEvents|Q
  (params (Key :type Key%20Structure))
  (bind _arrow1 (Variables|Default|GetArrow1))
  (bind _returnvalue (Math|Vector|GetForwardVector _arrow1))
  (:Pressed
    (bind _returnvalue_2 (Game|SpawnActorfromClass "/Game/Weapons/Knife.Knife_C" (Math|Transform|MakeTransform (Transformation|GetWorldLocation _arrow1) (Math|Rotator|MakeRotationfromAxes _returnvalue _returnvalue (Math|Vector|GetUpVector _arrow1)) "1,1,1") "Undefined" 0 0))
    (Physics|AddImpulse (Variables|/Game/Weapons/Knife.Knife_C|GetCube _returnvalue_2) (* _returnvalue 2e+03) "None" true)))

(event Input|KeyboardEvents|E
  (params (Key :type Key%20Structure))
  (:Pressed
    (Utilities|FlowControl|DoOnce false :!label _label
      (:Completed
        (if (not (AI|Components|NavMovement|IsFalling (Variables|Character|GetCharacterMovement)))
          (Character|LaunchCharacter (* (+ (* (Math|Vector|GetForwardVector (Variables|Default|GetCapsuleComponent)) (Variables|Default|GetForward/BackwardMovement)) (* (Math|Vector|GetRightVector (Variables|Default|GetCapsuleComponent)) (Variables|Default|GetRight/LeftMovement))) 1e+04) false false)))))
  (:Released
    (if (== (Variables|Default|GetCooldown) 0.0)
      (Variables|Default|SetCooldown 3.0)
      (Utilities|FlowControl|Delay 3.0)
      (goto _label Reset))))

(fn ConstructionScript)